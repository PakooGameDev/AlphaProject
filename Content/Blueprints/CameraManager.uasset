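; Top-down camera actor with a visible cursor, keyboard-style axis panning, screen-edge scrolling and mouse zoom.
; Inputs set a target location and clamped zoom, and Tick interpolates the actor and spring arm toward them.
; The arm's pitch target switches to a shallower angle when zoomed in close.
; Yaw rotation is gated on MouseIsPressed, which both middle-mouse press and release set to false.
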(event `self.ReceiveBeginPlay`
  (set `self.ZoomValue` (`SpringArmComponent.TargetArmLength` (`self.SpringArm`)))
  (set `self.CameraLocation` (`self.K2_GetActorLocation`))
  (set `self.CameraRotation` (`self.K2_GetActorRotation`))
  (set `PlayerController.bShowMouseCursor` true (`GameplayStatics.GetPlayerController` 0)))

(event `InputAxis|CameraZoom`
  (params (AxisValue :type "Float (single-precision)"))
  (set `self.ZoomValue` (`KismetMathLibrary.FClamp` (+ (* AxisValue (`self.ZoomSpeed`)) (`self.ZoomValue`)) 200.0 5000.0))
  (set `self.SpringArmRotation` (`KismetMathLibrary.SelectRotator` (struct :`Pitch` -30.0) (struct :`Pitch` -60.0) (< (`self.ZoomValue`) 500.0))))

(event `self.ReceiveTick`
  (params (DeltaSeconds :type "Float (single-precision)"))
  (bind _springarm (`self.SpringArm`))
  (bind _springarm_2 (`self.SpringArm`))
  (set `SpringArmComponent.TargetArmLength` (`KismetMathLibrary.FInterpTo` (`SpringArmComponent.TargetArmLength` _springarm) (`self.ZoomValue`) DeltaSeconds 2.0) _springarm)
  (`self.K2_SetActorLocation` (`KismetMathLibrary.VInterpTo` (`self.K2_GetActorLocation`) (`self.CameraLocation`) DeltaSeconds 10.0))
  (`SceneComponent.K2_SetRelativeRotation` _springarm_2 (`KismetMathLibrary.RInterpTo` (`SceneComponent.RelativeRotation` _springarm_2) (`self.SpringArmRotation`) DeltaSeconds 4.0) false false))

(event `InputAction|MouseWheelDownAction`
  (params (Key :type "Key Structure"))
  (:`Pressed`
    (set `self.MouseIsPressed` false))
  (:`Released`
    (set `self.MouseIsPressed` false)))

(event `InputAxis|MoveRight`
  (params (AxisValue :type "Float (single-precision)"))
  (set `self.CameraLocation` (+ (* AxisValue (`self.GetActorRightVector`) (`self.CameraSpeed`)) (`self.CameraLocation`))))

(event `InputAxis|CameraRotation`
  (params (AxisValue :type "Float (single-precision)"))
  (bind (_returnvalue_roll _returnvalue_pitch _returnvalue_yaw) (`KismetMathLibrary.BreakRotator` (`self.K2_GetActorRotation`)))
  (if (`self.MouseIsPressed`)
    (`self.K2_SetActorRotation` (`KismetMathLibrary.MakeRotator` 0.0 0.0 (`KismetMathLibrary.FClamp` (+ (* AxisValue (`self.CameraRotationSpeed`)) _returnvalue_yaw) -360.0 360.0)))))

(event `InputAxis|MoveForward`
  (params (AxisValue :type "Float (single-precision)"))
  (set `self.CameraLocation` (+ (* AxisValue (`self.GetActorForwardVector`) (`self.CameraSpeed`)) (`self.CameraLocation`))))

(event `InputAxis|CameraLocation`
  (params (AxisValue :type "Float (single-precision)"))
  (bind (_returnvalue_x _returnvalue_y) (`KismetMathLibrary.BreakVector2D` (`WidgetLayoutLibrary.GetViewportSize`)))
  (bind (_locationx _locationy) (`PlayerController.GetMousePosition` (`GameplayStatics.GetPlayerController` 0)))
  (bind _returnvalue (`KismetMathLibrary.MapRangeClamped` (/ _locationy _returnvalue_y) 0.0 1.0 -1.0 1.0))
  (bind _returnvalue_2 (`KismetMathLibrary.MapRangeClamped` (/ _locationx _returnvalue_x) 0.0 1.0 -1.0 1.0))
  (bind _returnvalue_3 (>= (`KismetMathLibrary.Abs` _returnvalue) 0.95))
  (bind _returnvalue_4 (+ (* (`self.GetActorRightVector`) (`self.CameraSpeed`) (`KismetMathLibrary.SelectFloat` -1.0 1.0 (< _returnvalue_2 0.0))) (`self.CameraLocation`)))
  (bind _returnvalue_5 (+ (* (`self.GetActorForwardVector`) (`self.CameraSpeed`) (`KismetMathLibrary.SelectFloat` 1.0 -1.0 (< _returnvalue 0.0))) (`self.CameraLocation`)))
  (if (>= (`KismetMathLibrary.Abs` _returnvalue_2) 0.95)
    (if _returnvalue_3
      (set `self.CameraLocation` _returnvalue_4)
      (set `self.CameraLocation` _returnvalue_5)
      (else
        (set `self.CameraLocation` _returnvalue_4)))
    (elif _returnvalue_3
      (set `self.CameraLocation` _returnvalue_5))))

(fn `UserConstructionScript`)